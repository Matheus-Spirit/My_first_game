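; BP_item is a pickup actor whose mesh is set from the ItemModelPlace variable in the construction script.
; Its PickUp event prints a debug message and plays the Shrink timeline, which lerps the model's world scale from one to zero.
; A DoOnce on the timeline's update plays a pickup sound a single time, then destroys the actor after a short delay.
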(event EventBeginPlay)

(event Collision|EventActorBeginOverlap
  (params (OtherActor :type Actor%20Object%20Reference)))

(event EventTick
  (params (DeltaSeconds :type Float%20%28single-precision%29)))

(event EventPickUp
  (Development|PrintString "item picked")
  (bind _shrink__timeline (Timeline|Shrink Play)
    (:Update
      (Transformation|SetWorldScale3D (Variables|Default|GetitemModel) (Math|Conversions|ToVector(Float) (Math|Float|Lerp 1.0 0.0 _shrink__timeline)))
      (Utilities|FlowControl|DoOnce false
        (:Completed
          (Audio|PlaySound2D "/Engine/VREditor/Sounds/UI/Dockable_Window_Pick_Up.Dockable_Window_Pick_Up" 1.0 1.0 0.0 0 0)
          (Utilities|FlowControl|Delay 0.4)
          (Actor|DestroyActor))))))

(fn ConstructionScript
  (Components|StaticMesh|SetStaticMesh (Variables|Default|GetitemModel) (Variables|Default|GetitemModelPlace)))